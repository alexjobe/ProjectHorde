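; BP_ShooterCharacter_Player is the player's shooter character, adding the on-screen HUD on top of its parent class.
; On BeginPlay it runs the parent logic, then, only if locally controlled, creates crosshair, health and ammo widgets and adds each to the viewport.
; The construction script only calls the parent version.
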(event `self.ReceiveBeginPlay`
  (`parent.ReceiveBeginPlay`)
  (if (`self.IsLocallyControlled`)
    (`|ExecutionSequence`
      (:`then_0`
        (bind _returnvalue (`|CreateWidget` "/Game/UI/WBP_Crosshair.WBP_Crosshair_C"))
        (`UserWidget.AddToViewport` _returnvalue 0))
      (:`then_1`
        (bind _returnvalue_2 (`|CreateWidget` "/Game/UI/WBP_Health.WBP_Health_C"))
        (`UserWidget.AddToViewport` _returnvalue_2 0))
      (:`then_2`
        (bind _returnvalue_3 (`|CreateWidget` "/Game/UI/WBP_Ammo.WBP_Ammo_C"))
        (`UserWidget.AddToViewport` _returnvalue_3 0)))))

(fn `UserConstructionScript`
  (`parent.UserConstructionScript`))